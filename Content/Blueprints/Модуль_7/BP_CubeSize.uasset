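; BP_CubeSize is an actor Blueprint that shrinks itself each time another actor begins overlapping it.
; BeginPlay caches five percent of the starting scale as SizeVector.
; Each overlap calls the parent handler, then subtracts that fixed step from the current scale, so shrinkage is linear and has no lower limit.
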(event `self.ReceiveBeginPlay`
  (bind _output_get (set `self.SizeVector` (* (`self.GetActorScale3D`) 0.05))))

(event `self.ReceiveActorBeginOverlap`
  (params (OtherActor :type "Actor Object Reference"))
  (`parent.ReceiveActorBeginOverlap` OtherActor)
  (`self.SetActorScale3D` (- (`self.GetActorScale3D`) (stale `self.ReceiveBeginPlay` _output_get))))

(fn `UserConstructionScript`
  (`parent.UserConstructionScript`))