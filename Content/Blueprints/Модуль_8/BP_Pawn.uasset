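; BP_Pawn is a player pawn that slides sideways and spawns a ball, apparently as a paddle.
; MoveRight input shifts it in fixed, unswept Y-axis steps opposite to the axis sign, without delta-time scaling.
; On BeginPlay, SpawnBall creates a BP_ball1 at the Sphere component, stores it as PlayingBall and binds its OnDead dispatcher.
; BeginPlay also binds OnDead on a separate spawnBall reference to an empty handler.
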(event `InputAxis|MoveRight`
  (params (AxisValue :type "Float (single-precision)"))
  (if (< AxisValue 0.0)
    (`self.K2_AddActorWorldOffset` (0.0 50.0 0.0))))

(event `InputAxis|MoveRight`
  (params (AxisValue :type "Float (single-precision)"))
  (if (> AxisValue 0.0)
    (`self.K2_AddActorWorldOffset` (0.0 -50.0 0.0))))

(event `self.ReceiveBeginPlay`
  (bind _output_get (`self.SpawnBall`))
  (add `/Game/Blueprints/BP_ball1.OnDead` _output_get (delegate `OnDead_Event_0`)))

(event `OnDead_Event_0`)

(fn `SpawnBall`
  (returns (Output_Get :type "/Game/Blueprints/BP_ball1 Object Reference"))
  (bind _returnvalue (`|SpawnActorFromClass` "/Game/Blueprints/BP_ball1.BP_ball1_C" (`SceneComponent.K2_GetComponentToWorld` (`self.Sphere`)) "AlwaysSpawn" "OverrideRootScale" null null))
  (bind _output_get (set `self.PlayingBall` _returnvalue))
  (add `/Game/Blueprints/BP_ball1.OnDead` _output_get (`|CreateDelegate` :!event `SpawnDefaultController`)))

(fn `UserConstructionScript`)