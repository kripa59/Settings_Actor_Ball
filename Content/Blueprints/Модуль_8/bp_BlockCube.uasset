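; bp_BlockCube is a breakable block that reacts to hits from BP_ball1.
; Each ball hit decrements HitCount, and while hits remain the Cube mesh switches its material to M_Rock_Sandstone as damage feedback.
; When the count runs out, it destroys its own hit component rather than the actor and adds a child actor component in the same event.
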(event `self.ReceiveHit`
  (params (MyComp :type "PrimitiveComponent Object Reference") (Other :type "Actor Object Reference") (OtherComp :type "PrimitiveComponent Object Reference") (bSelfMoved :type Boolean) (HitLocation :type "Vector Structure") (HitNormal :type "Vector Structure") (NormalImpulse :type "Vector Structure") (Hit :type "HitResult Structure (by ref)"))
  (cast `/Game/Blueprints/BP_ball1` Other)
  (set `self.HitCount` (- (`self.HitCount`) 1))
  (if (<= (`self.HitCount`) 0)
    (`ActorComponent.K2_DestroyComponent` MyComp)
    (`AddComponent|NODE_AddChildActorComponent-0`)
    (else
      (`PrimitiveComponent.SetMaterial` (`self.Cube`) 0 "/Game/StarterContent/Materials/M_Rock_Sandstone.M_Rock_Sandstone"))))

(fn `UserConstructionScript`)